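; Game mode that runs a pre-fight countdown before starting the boss match.
; On BeginPlay it shows the countdown widget with UI-only input, then a looping one-second timer updates it and decrements the seconds.
; At zero it clears the timer, briefly shows the fight text, removes the widget, restores game-only input and calls StartGame on the boss's AI controller.
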(event `self.ReceiveBeginPlay`
  (bind _returnvalue (`GameplayStatics.GetPlayerController` 0))
  ;[1 1 1] Game started, start countdown
  (bind _returnvalue_2 (`|CreateWidget` "/Game/Game/Widgets/WB_Countdown.WB_Countdown_C" _returnvalue))
  (bind _output_get (set `self.CountdownUI` _returnvalue_2))
  (`UserWidget.AddToViewport` _output_get 0)
  (`WidgetBlueprintLibrary.SetInputMode_UIOnlyEx` _returnvalue _returnvalue_2)
  (`self.BeginCountdown`))

(event `BeginCountdown`
  ;[1 1 1] Match countdown
  (bind _returnvalue (`KismetSystemLibrary.K2_SetTimerDelegate` (delegate `CountdownTimer`) 1.0 true))
  (set `self.CountdownTimerHandle` _returnvalue))

(event `CountdownTimer`
  (bind _countdownui (`self.CountdownUI`))
  ;[1 1 1] Match countdown
  (`/Game/Game/Widgets/WB_Countdown.UpdateCountdownTimer` (`self.CountdownUI`) (`self.TimerSeconds`))
  (if (== (`self.TimerSeconds`) 0)
    (`KismetSystemLibrary.K2_ClearAndInvalidateTimerHandle` (`self.CountdownTimerHandle`))
    (`Widget.SetVisibility` (`/Game/Game/Widgets/WB_Countdown.CountdownGroup` _countdownui) "Hidden")
    (`Widget.SetVisibility` (`/Game/Game/Widgets/WB_Countdown.FightText` _countdownui) "Visible")
    (`KismetSystemLibrary.Delay` 1.0)
    (`Widget.RemoveFromParent` (`self.CountdownUI`))
    (`self.MatchStart`)
    (else
      (set `self.TimerSeconds` (- (`self.TimerSeconds`) 1) :!label _label))))

(event `InitialCountdownSubstraction`
  ;[1 1 1] Match countdown
  (goto _label))

(event `MatchStart`
  (`WidgetBlueprintLibrary.SetInputMode_GameOnly` (`GameplayStatics.GetPlayerController` 0))
  (bind _returnvalue (`GameplayStatics.GetActorOfClass` "/Game/Game/Blueprints/BP_Boss.BP_Boss_C"))
  (bind _asbp_boss_controller (cast `/Game/Game/Blueprints/BP_BossController` (`Pawn.GetController` _returnvalue)))
  (`/Game/Game/Blueprints/BP_BossController.StartGame` _asbp_boss_controller))

(fn `UserConstructionScript`)