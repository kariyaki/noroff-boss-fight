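; AI controller for the boss that starts its behavior tree on StartGame and seeds the blackboard with health and the boss's dash range.
; Once started, perception updates feed sight and prediction handlers that only react to the player.
; Sight sets or clears the target and flags the match as begun.
; Losing sight requests an AI prediction event, whose result stores the player's predicted location in the blackboard.
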(event `StartGame`
  ;[1 1 1] Start behaviour tree after countdown
  (set `self.GameStarted?` true)
  (`self.RunBehaviorTree` "/Game/Game/Blueprints/BT_Boss.BT_Boss")
  (`self.UpdateCurrentHealth` 100.0)
  (bind _asbp_boss (cast `/Game/Game/Blueprints/BP_Boss` (`self.K2_GetPawn`)))
  (`BlackboardComponent.SetValueAsFloat` (`self.Blackboard`) "DashRange" (`/Game/Game/Blueprints/BP_Boss.MaxDashRange` _asbp_boss)))

(event `self.AIPerception.OnTargetPerceptionUpdated`
  (params (Actor :type "Actor Object Reference") (Stimulus :type "AIStimulus Structure"))
  ;[1 1 1] AIPerception logic
  (if (`self.GameStarted?`)
    (`self.HandleSightSense` Actor Stimulus)
    (`self.HandlePredictionSense` Actor Stimulus)))

(fn `HandlePredictionSense`
  (params (Actor :type "Actor Object Reference") (Stimulus :type "AIStimulus Structure"))
  (bind (_stimulus_age _stimulus_expirationage _stimulus_strength _stimulus_stimuluslocation) (break `AIStimulus` (`local.Stimulus`)))
  ;[1 1 1] The boss predicts where the player is
  (bind _returnvalue (`AIPerceptionSystem.GetSenseClassForStimulus` Stimulus))
  (if (== _returnvalue "/Script/AIModule.AISense_Prediction")
    (if (== (`local.Actor`) (`GameplayStatics.GetPlayerCharacter` 0))
      (`BlackboardComponent.SetValueAsVector` (`self.Blackboard`) "PredictedLocation" _stimulus_stimuluslocation)
      (else
        (return)))
    (else
      (return))))

(fn `HandleSightSense`
  (params (Actor :type "Actor Object Reference") (Stimulus :type "AIStimulus Structure"))
  (bind (_stimulus_age _stimulus_expirationage _stimulus_strength _stimulus_stimuluslocation _stimulus_receiverlocation _stimulus_tag _stimulus_bsuccessfullysensed) (break `AIStimulus` (`local.Stimulus`)))
  ;[1 1 1] Boss sees someone, set target and targetlocation if the seen actor is the player. If the boss lost sight of the player, initiate prediction
  (bind _returnvalue (`AIPerceptionSystem.GetSenseClassForStimulus` Stimulus))
  (if (== _returnvalue "/Script/AIModule.AISense_Sight")
    (if (== (`local.Actor`) (`GameplayStatics.GetPlayerCharacter` 0))
      ;;[1 1 1] Indicated the boss has seen the player atleast once
      (`BlackboardComponent.SetValueAsBool` (`self.Blackboard`) "MatchBegun" true)
      (`BlackboardComponent.SetValueAsObject` (`self.Blackboard`) "TargetActor" (`KismetMathLibrary.SelectObject` (`GameplayStatics.GetPlayerCharacter` 0) null _stimulus_bsuccessfullysensed))
      (if (not _stimulus_bsuccessfullysensed)
        (`AISense_Prediction.RequestPawnPredictionEvent` (`self.K2_GetPawn`) (`GameplayStatics.GetPlayerCharacter` 0) 1.0))
      (else
        (return)))
    (else
      (return))))

(fn `UpdateCurrentHealth`
  (params (CurrentHealth :type "Float (single-precision)"))
  (bind _blackboard (`self.Blackboard`))
  (`/Engine/EditorBlueprintResources/StandardMacros.IsValid` _blackboard
    (:`Is Valid`
      (`BlackboardComponent.SetValueAsFloat` _blackboard "CurrentHP" CurrentHealth))))

(fn `UserConstructionScript`)