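; Boss enemy character that fights the player with a punch and a timed jump attack, and quits the game shortly after it is killed.
; Tick writes melee and jump-attack range checks against the player to the Blackboard.
; Attack plays a punch montage while damaging the target, SmashAttack toggles timed state flags, and hits report touch events.
; Damage updates an on-screen, color-changing health bar and passes health to BP_BossController.
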(event `self.ReceiveBeginPlay`
  ;[1 1 1] Setup healthbar
  (bind _returnvalue (`|CreateWidget` "/Game/Game/Widgets/WB_BossHealth.WB_BossHealth_C"))
  (`UserWidget.AddToViewport` _returnvalue 0)
  (set `self.BossHealth` _returnvalue)
  (`self.UpdateHealth` (`self.Health`))
  (bind _asbp_boss_controller (cast `/Game/Game/Blueprints/BP_BossController` (`self.GetController`)))
  (set `self.BossController` _asbp_boss_controller))

(event `self.ReceiveTick`
  (params (DeltaSeconds :type "Float (single-precision)"))
  (`|ExecutionSequence`
    (:`then_0`
      ;[1 1 1] Check to see if player is within melee range
      (`/Engine/EditorBlueprintResources/StandardMacros.IsValid` (`AIBlueprintHelperLibrary.GetBlackboard` null)
        (:`Is Valid`
          (`BlackboardComponent.SetValueAsBool` (`AIBlueprintHelperLibrary.GetBlackboard` null) "PlayerInMeleeRange" (<= (`self.GetDistanceTo` self (`GameplayStatics.GetPlayerCharacter` 0)) (`self.MeleeRange`))))))
    (:`then_1`
      ;[1 1 1] Is the player in jumpattack range?
      (`/Engine/EditorBlueprintResources/StandardMacros.IsValid` (`AIBlueprintHelperLibrary.GetBlackboard` null)
        (:`Is Valid`
          (`BlackboardComponent.SetValueAsBool` (`AIBlueprintHelperLibrary.GetBlackboard` null) "CanJumpAttack?" (and (>= (`self.GetDistanceTo` self (`GameplayStatics.GetPlayerCharacter` 0)) (- (`self.JumpAttackRange`) 100.0)) (<= (`self.GetDistanceTo` self (`GameplayStatics.GetPlayerCharacter` 0)) (+ (`self.JumpAttackRange`) 300.0)))))))))

(event `/Game/Game/Blueprints/BPI_Character.Attack`
  (params (OtherActor :type "Object Object Reference") (Damage :type "Float (double-precision)"))
  ;[1 1 1] Attack Player
  (if (not (`self.IsAttacking?`))
    (set `self.IsAttacking?` true)
    (`|PlayMontage` (`self.Mesh`) "/Game/Characters/Mannequins/Animations/Manny/Mutant_Punch_Montage.Mutant_Punch_Montage"
      (:`then`
        (message `/Game/Game/Blueprints/BPI_Character.TakeDamage` OtherActor Damage))
      (:`OnCompleted`
        (set `self.IsAttacking?` false)))))

(event `/Game/Game/Blueprints/BPI_Character.TakeDamage`
  (params (Damage :type "Float (double-precision)"))
  (bind _returnvalue (- (`self.Health`) Damage))
  ;[1 1 1] Boss takes damage
  (if (<= _returnvalue 0.0)
    (set `self.Dead?` true)
    (`KismetSystemLibrary.PrintString` "YOU KILLED THE BOSS! YEY!")
    (`KismetSystemLibrary.Delay` 3.0)
    (`KismetSystemLibrary.QuitGame` null "Quit")
    (else
      (bind _output_get (set `self.Health` _returnvalue))
      (`self.UpdateHealth` _output_get))))

(event `self.ReceiveHit`
  (params (MyComp :type "PrimitiveComponent Object Reference") (Other :type "Actor Object Reference") (OtherComp :type "PrimitiveComponent Object Reference") (bSelfMoved :type Boolean) (HitLocation :type "Vector Structure") (HitNormal :type "Vector Structure") (NormalImpulse :type "Vector Structure") (Hit :type "HitResult Structure (by ref)"))
  ;[1 1 1] Start Touch event on hit
  (`AISense_Touch.ReportTouchEvent` self Other)
  (`/Game/Game/Blueprints/BP_BossController.ResetTouch` (`self.BossController`)))

(event `SmashAttack`
  ;[1 1 1] Start Jump Attack
  (set `self.PreparingToJumpAttack?` true)
  (`KismetSystemLibrary.Delay` 1.0)
  (set `self.IsJumpAttacking?` true)
  (`KismetSystemLibrary.Delay` 2.0)
  (set `self.IsJumpAttacking?` false)
  (set `self.PreparingToJumpAttack?` false))

(fn `UpdateHealth`
  (params (InPercent :type "Float (single-precision)"))
  (bind _inpercent (`local.InPercent`))
  (bind _healthbar (`/Game/Game/Widgets/WB_BossHealth.HealthBar` (`self.BossHealth`)))
  ;[1 1 1] Update healthbar and BT health information
  (bind _asbp_boss_controller (cast `/Game/Game/Blueprints/BP_BossController` (`self.GetController`)))
  (`/Game/Game/Blueprints/BP_BossController.UpdateCurrentHealth` _asbp_boss_controller _inpercent)
  (`ProgressBar.SetPercent` (`/Game/Game/Widgets/WB_BossHealth.HealthBar` (`self.BossHealth`)) (/ _inpercent 100.0))
  (if (< (`local.InPercent`) 35.0)
    (`ProgressBar.SetFillColorAndOpacity` _healthbar (struct :`R` 1.0 :`G` 0.876225 :`B` 0.110122 :`A` 1.0))
    (elif (< (`local.InPercent`) 66.0)
      (`ProgressBar.SetFillColorAndOpacity` _healthbar (struct :`R` 0.019134 :`G` 0.307292 :`B` 0.019046 :`A` 1.0)))))

(fn `UserConstructionScript`)